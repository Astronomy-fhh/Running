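; Game Instance Blueprint for the Running game that owns a persistent screen transition widget and handles level changes.
; On Init it creates and stores a UI_Transition widget.
; Transition In and Transition Out add the widget to the viewport if needed and trigger the matching transition.
; OpenLevel starts the transition in, waits briefly, then opens the given level by object reference.
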(event Custom|Open%20Level
  (params (Level :type World%20Soft%20Object%20Reference))
  (CallFunction|Transitionin)
  (Utilities|FlowControl|Delay 0.1)
  (Game|OpenLevel(byObjectReference) Level))

(event EventInit
  (Utilities|FlowControl|Sequence
    (:then_0
      (bind _returnvalue (UserInterface|CreateWidget "/Game/Running/UI/UI_Transition.UI_Transition_C"))
      (Variables|Default|SetUI%20Transition _returnvalue))))

(fn Transitionin
  (if (UserInterface|Viewport|IsinViewport (Variables|Default|GetUI%20Transition))
    _
    (else
      (UserInterface|Viewport|AddtoViewport (Variables|Default|GetUI%20Transition) 0)))
  (Default|Transitionin (Variables|Default|GetUI%20Transition)))

(fn TransitionOut
  (if (UserInterface|Viewport|IsinViewport (Variables|Default|GetUI%20Transition))
    _
    (else
      (UserInterface|Viewport|AddtoViewport (Variables|Default|GetUI%20Transition) 0)))
  (Default|TransitionOut (Variables|Default|GetUI%20Transition)))