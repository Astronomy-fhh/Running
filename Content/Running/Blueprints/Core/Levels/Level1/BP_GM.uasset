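; Level 1 game manager for the running game that starts and restarts runs and drives the player stats HUD.
; A looping timer waits for a valid spawner, supplied by its generation-completed event, then teleports the character to its start point and starts running after a delay.
; BackStart resets stats, teleports back and recenters the spawner's path before restarting.
; Tick pushes score and fly speed against max speed into the HUD.
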(event Custom|Spawner%20Gen%20Completed
  (params (Spawner :type BP%20Spawner%20Object%20Reference))
  (Variables|Default|SetSpawner Spawner))

(event Custom|Set%20Start%20Point
  (bind _spawner (Variables|Default|GetSpawner)
    (:then
      (bind _center__start_point (Default|GetStartPoint _spawner))
      (Variables|Default|SetCenter%20%20Start%20Point _center__start_point)
      (bind _asbp_running_character (Utilities|Casting|CastToBP_RunningCharacter (Game|GetPlayerCharacter 0)))
      (Variables|Default|SetCharacter _asbp_running_character)
      (Transformation|Teleport (Variables|Default|GetCharacter) (Variables|Default|GetCenter%20%20Start%20Point) "0, 0, 0")
      (Utilities|Time|ClearandInvalidateTimerbyHandle (Variables|Default|GetSet%20Start%20Point%20Loop))
      (Utilities|FlowControl|Delay 2.0)
      (Default|StartRunning (Variables|Default|GetCharacter) (Variables|Default|GetSpawner)))
    (:else)))

(event Custom|Back%20Start
  (Default|Reset (Variables|/Game/Running/Characters/BP_RunningCharacter.BP_RunningCharacter_C|GetBPC_Player_Stats (Variables|Default|GetCharacter)))
  (Transformation|Teleport (Variables|Default|GetCharacter) (Variables|Default|GetCenter%20%20Start%20Point) "0, 0, 0")
  (Default|ToCenterPath (Variables|Default|GetSpawner))
  (Utilities|FlowControl|Delay 2.0)
  (Default|StartRunning (Variables|Default|GetCharacter) (Variables|Default|GetSpawner)))

(event EventTick
  (params (DeltaSeconds :type Float%20%28single-precision%29))
  (bind _character (Variables|Default|GetCharacter))
  (bind _charactermovement (Variables|/Script/Engine.Character|GetCharacterMovement _character))
  (bind _maxflyspeed (Variables|/Script/Engine.CharacterMovementComponent|GetMaxFlySpeed _charactermovement))
  (Variables|Default|GetUI_Player_Stats
    (:then
      (bind _character_2 (Variables|Default|GetCharacter)
        (:then
          (Variables|/Script/UMG.TextBlock|SetText (Variables|/Game/Running/UI/UI_Player_Info.UI_Player_Info_C|GetScoreText (Variables|Default|GetUI_Player_Stats)) (Utilities|Text|ToText(Float) (Variables|/Game/Running/Blueprints/Comp/BPC_Player_Stats.BPC_Player_Stats_C|GetScore (Variables|/Game/Running/Characters/BP_RunningCharacter.BP_RunningCharacter_C|GetBPC_Player_Stats _character_2)) "HalfToEven"))
          (Variables|/Script/UMG.TextBlock|SetText (Variables|/Game/Running/UI/UI_Player_Info.UI_Player_Info_C|GetSpeedText (Variables|Default|GetUI_Player_Stats)) (Utilities|Text|FormatText "{cur}/{max}" _maxflyspeed (Variables|/Game/Running/Blueprints/Comp/BPC_Player_Stats.BPC_Player_Stats_C|GetMaxSpeed (Variables|/Game/Running/Characters/BP_RunningCharacter.BP_RunningCharacter_C|GetBPC_Player_Stats _character_2))))
          (Progress|SetPercent (Variables|/Game/Running/UI/UI_Player_Info.UI_Player_Info_C|GetSpeedProgressBar (Variables|Default|GetUI_Player_Stats)) (/ _maxflyspeed (Variables|/Game/Running/Blueprints/Comp/BPC_Player_Stats.BPC_Player_Stats_C|GetMaxSpeed (Variables|/Game/Running/Characters/BP_RunningCharacter.BP_RunningCharacter_C|GetBPC_Player_Stats _character_2)))))
        (:else)))
    (:else)))

(event EventBeginPlay
  (Utilities|FlowControl|Sequence
    (:then_0
      (bind _returnvalue (UserInterface|CreateWidget "/Game/Running/UI/UI_Player_Info.UI_Player_Info_C"))
      (bind _output_get (Variables|Default|SetUI_Player_Stats _returnvalue))
      (UserInterface|Viewport|AddtoViewport _output_get 0))
    (:then_1
      (bind _returnvalue_2 (Utilities|Time|SetTimerbyEvent (delegate Custom|Set%20Start%20Point) 0.1 true))
      (Variables|Default|SetSet%20Start%20Point%20Loop _returnvalue_2))))

(fn ConstructionScript)