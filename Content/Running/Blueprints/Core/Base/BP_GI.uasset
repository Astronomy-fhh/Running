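; Game instance that handles level changes behind a transition screen.
; Init creates a single UI_Transition widget and keeps a reference to it.
; OpenLevel adds that widget to the viewport through TransitionIn, waits a fixed delay, then opens the requested level by object reference.
; TransitionOut removes the widget, and both transition functions check viewport state first to avoid redundant adds or removals.
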(event Custom|Open%20Level
  (params (Level :type World%20Soft%20Object%20Reference))
  (CallFunction|Transitionin)
  (Utilities|FlowControl|Delay 2.0)
  (Game|OpenLevel(byObjectReference) Level))

(event EventInit
  (Utilities|FlowControl|Sequence
    (:then_0
      (bind _returnvalue (UserInterface|CreateWidget "/Game/Running/UI/UI/UI_Transition.UI_Transition_C"))
      (Variables|Default|SetUI%20Transition _returnvalue))))

(fn Transitionin
  (if (not (UserInterface|Viewport|IsinViewport (Variables|Default|GetUI%20Transition)))
    (UserInterface|Viewport|AddtoViewport (Variables|Default|GetUI%20Transition) 0)))

(fn TransitionOut
  (if (UserInterface|Viewport|IsinViewport (Variables|Default|GetUI%20Transition))
    (Widget|RemovefromParent (Variables|Default|GetUI%20Transition))))