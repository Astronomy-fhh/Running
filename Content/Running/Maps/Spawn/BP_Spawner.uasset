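; BP_Spawner procedurally builds an obstacle course with a passable route for a lane-based running map.
; On BeginPlay it splits the Path bounds into an odd number of lanes along X, then fills each with random barriers spaced by measured bounds and random gaps.
; It carves a route from the center lane, box-tracing and destroying barriers while randomly hopping to adjacent lanes, then notifies BP_GM.
; It also provides start-point and lane-movement helpers.
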(event EventBeginPlay
  (Utilities|FlowControl|Sequence
    (:then_0
      ;[1 1 1] 初始化一些坐标
      (Init|InitXYZ)
      (Init|InitStartPoint)
      (Init|InitPathNY)
      (CallFunction|InitCenterPoint))
    (:then_1
      ;[1 1 1] 生成障碍物
      (Barrier|SpawnBarriers))
    (:then_2
      ;[1 1 1] 生成一条通路 清理掉通路上的障碍物
      (Passer|SpawnPasserRoute))
    (:then_3
      ;[1 1 1] 通知生成完成
      (bind _asbp_gm (Utilities|Casting|CastToBP_GM (Game|GetGameMode)))
      (Default|SpawnerGenCompleted _asbp_gm self))))

(fn ConstructionScript)

(fn SpawnBarries
  (Utilities|FlowControl|Sequence
    (:then_0
      (bind _returnvalue (Game|SpawnActorfromClass "/Game/Running/Maps/Spawn/Barriers/BPC_Barrier_Blue.BPC_Barrier_Blue_C" (Math|Transform|MakeTransform "0, 0, 0" "0, 0, 0" "1.000000,1.000000,1.000000") "AlwaysSpawn" "MultiplyWithRoot" 0 0)))
    (:then_1)
    (:then_2
      (for _index (range 0 200)
        (Game|SpawnActorfromClass "/Game/Running/Maps/Spawn/Barriers/BPC_Barrier_Blue.BPC_Barrier_Blue_C" (Math|Transform|MakeTransform (Math|Vector|MakeVector (Math|Float|Lerp 0.0 0.0 (Math|Random|RandomFloat)) (Math|Float|Lerp 0.0 0.0 (Math|Random|RandomFloat)) 0.0) (Math|Rotator|MakeRotator 0.0 0.0 (Math|Float|Lerp 0.0 1.8e+02 (Math|Random|RandomFloat))) (Math|Conversions|ToVector(Float) (Math|Float|Lerp 0.5 2.0 (Math|Random|RandomFloat)))) "DontSpawnIfColliding" "MultiplyWithRoot" 0 0)))))

(fn InitXYZ
  (Variables|Path|SetPath%20XYZ (.BoxExtent (Collision|GetComponentBounds (Variables|Default|GetPath)))))

(fn InitStartPoint
  (bind _path (Variables|Default|GetPath))
  (bind _path_xyz (Variables|Path|GetPath%20XYZ))
  (bind _returnvalue (Transformation|GetWorldLocation _path))
  (Variables|Point|SetBase%20Point (Math|Vector|MakeVector (- (.x _returnvalue) (.x _path_xyz)) (- (.y _returnvalue) (.y _path_xyz)) (.z _returnvalue)))
  (CallFunction|DebugSphere (Variables|Point|GetBase%20Point)))

(fn DebugSphere
  (params (Center :type Vector))
  (if (Variables|Debug|GetDebug%20Draw)
    (Rendering|Debug|DrawDebugSphere Center 1e+02 12 "(R=1.000000,G=0.218750,B=0.910548,A=1.000000)" 1e+02)))

(fn InitPathNY
  (bind _output_get (Variables|Path|SetPath%20N (+ (* (/ (Math|Integer|SelectInt (Variables|Path|GetPath%20N) 1 (> (Variables|Path|GetPath%20N) 0)) 2) 2) 1)))
  (Variables|Path|SetPath%20Y%20Size (/ (* (.y (Variables|Path|GetPath%20XYZ)) 2.0) _output_get))
  (bind _output_get_2 (Variables|Path|SetCenter%20Path%20N (/ (Variables|Path|GetPath%20N) 2)))
  (Variables|Path|SetCurrent%20Path%20N _output_get_2))

(fn DrawDebugMid
  (if (Variables|Debug|GetDebug%20Draw)
    (for _index (range 0 (Variables|Path|GetPath%20N))
      (Rendering|Debug|DrawDebugArrow (+ (Variables|Point|GetBase%20Point) (Math|Vector|MakeVector 0.0 (* _index (Variables|Path|GetPath%20Y%20Size)) 1e+02)) (+ (+ (Variables|Point|GetBase%20Point) (Math|Vector|MakeVector 0.0 (* _index (Variables|Path|GetPath%20Y%20Size)) 1e+02)) (Math|Vector|MakeVector (* (.x (Variables|Path|GetPath%20XYZ)) 2.0) 0.0 0.0)) 1e+02 "(R=0.284579,G=0.428250,B=1.000000,A=1.000000)" 1e+03 0.0))))

(fn InitCenterPoint
  (bind _output_get (Variables|Point|SetCenter%20%20Start%20Point (+ (Variables|Point|GetBase%20Point) (Math|Vector|MakeVector (Variables|Path|GetStart%20Base%20X) (+ (* (/ (- (Variables|Path|GetPath%20N) 1) 2) (Variables|Path|GetPath%20Y%20Size)) (/ (Variables|Path|GetPath%20Y%20Size) 2.0)) (* (.z (Variables|Path|GetPath%20XYZ)) 2.0)))))
  (CallFunction|DebugSphere _output_get))

(fn GetRandomPathN)

(fn ToPathRight
  (if (<= (+ (Variables|Path|GetCurrent%20Path%20N) 1) (- (Variables|Path|GetPath%20N) 1))
    (Variables|Path|SetCurrent%20Path%20N (+ (Variables|Path|GetCurrent%20Path%20N) 1))
    (return true)
    (else
      (return false))))

(fn ToPathLeft
  (if (>= (- (Variables|Path|GetCurrent%20Path%20N) 1) 0)
    (Variables|Path|SetCurrent%20Path%20N (- (Variables|Path|GetCurrent%20Path%20N) 1))
    (return true)
    (else
      (return false))))

(fn RangdomtoPath
  (if (Math|Random|RandomBool)
    (bind _success (Path|ToPathRight))
    (if (not _success)
      (Path|ToPathLeft))
    (else
      (bind _success_2 (Path|ToPathLeft))
      (if (not _success_2)
        (Path|ToPathRight)))))

(fn GetCurrenPathY
  (bind _y (Path|GetPathY (Variables|Path|GetCurrent%20Path%20N)))
  (return _y))

(fn SpawnPasserRoute
  (Variables|Passer|SetPasser%20Spawn%20Base%20Point (Variables|Point|GetCenter%20%20Start%20Point))
  (bind _output_get (Variables|Default|SetPasser%20Spawn%20Loop true))
  (while _output_get
    (Passer|PasserClean)))

(fn SpawnBarriers
  (for _index (range 0 (- (Variables|Path|GetPath%20N) 1))
    (Barrier|SpawnBarrierPathOne _index)))

(fn SpawnBarrierPathOne
  (params (Path%20Index :type Integer))
  (bind _center__start_point (Variables|Point|GetCenter%20%20Start%20Point))
  (bind (_x _y _z) (Math|Vector|BreakVector _center__start_point))
  (bind _y_2 (Path|GetPathY Path%20Index))
  (Variables|Barrier|SetSpawn%20Barrier%20Base%20Point (Math|Vector|MakeVector _x _y_2 _z))
  (bind _output_get (Variables|Barrier|SetSpawn%20Barrier%20Loop true))
  (while _output_get
    (Barrier|SpawnBarrier)))

(fn GetPathY
  (params (Path%20Index :type Integer))
  (return (+ (* (Variables|Path|GetPath%20Y%20Size) Path%20Index) (/ (Variables|Path|GetPath%20Y%20Size) 2.0) (.Y (Math|Vector|BreakVector (Variables|Point|GetBase%20Point))))))

(fn SpawnBarrier
  (Utilities|FlowControl|Sequence
    (:then_0
      ;[1 1 1] 确定生成的障碍物类型
      (LocalVariables|SetActor (.OutItem (Utilities|Array|Random (Variables|Barrier|GetBarriers)))))
    (:then_1
      ;[1 1 1] 确定旋转角度
      (LocalVariables|SetRotation%20Z (Math|Float|SelectFloat (Math|Float|Lerp -2e+01 2e+01 (Math|Random|RandomFloat)) 0.0 (< (Math|Random|RandomFloat) (Variables|Barrier|GetBarrier%20Rotate%20Z%20Rate)))))
    (:then_2
      ;[1 1 1] 生成障碍
      (bind _returnvalue (Game|SpawnActorfromClass (LocalVariables|GetActor) (Math|Transform|MakeTransform (Variables|Barrier|GetSpawn%20Barrier%20Base%20Point) (Math|Rotator|MakeRotator 0.0 0.0 (LocalVariables|GetRotation%20Z)) "1.000000,1.000000,1.000000") "Undefined" "MultiplyWithRoot" 0 0))
      (bind _output_get (LocalVariables|SetSpawned%20Actor _returnvalue))
      (LocalVariables|SetActor%20XYZ (* (.BoxExtent (Collision|GetActorBounds _output_get false false)) 2.0)))
    (:then_3
      ;[1 1 1] 是否已经到达X边界
      (if (> (+ (.x (Variables|Barrier|GetSpawn%20Barrier%20Base%20Point)) (.x (LocalVariables|GetActor%20XYZ))) (+ (.x (Variables|Point|GetBase%20Point)) (* (.x (Variables|Path|GetPath%20XYZ)) 2.0)))
        (Actor|DestroyActor (LocalVariables|GetSpawned%20Actor))
        (Variables|Barrier|SetSpawn%20Barrier%20Loop false)
        (return)))
    (:then_4
      ;[1 1 1] 基于基础点 偏移一下生成的障碍物的位置
      (Transformation|AddActorWorldOffset (LocalVariables|GetSpawned%20Actor) (Math|Vector|MakeVector (/ (.x (LocalVariables|GetActor%20XYZ)) 2.0) 0.0 0.0)))
    (:then_5
      ;[1 1 1] 更新新的生成基准点
      (Variables|Barrier|SetSpawn%20Barrier%20Base%20Point (+ (Variables|Barrier|GetSpawn%20Barrier%20Base%20Point) (Math|Vector|MakeVector (+ (.x (LocalVariables|GetActor%20XYZ)) (Math|Float|Lerp (Variables|Barrier|GetBarrier%20Gap%20Base%20X) (* (Variables|Barrier|GetBarrier%20Gap%20Base%20X) (Variables|Barrier|GetBarrier%20Gap%20Mu%20Dia)) (Math|Random|RandomFloat))) 0.0 0.0))))
    (:then_6
      ;[1 1 1] 继续生成
      (return))))

(fn PasserClean
  (params (Index :type Integer))
  (bind _passer_xyz (Variables|Passer|GetPasser%20XYZ))
  (Utilities|FlowControl|Sequence
    (:then_0
      ;[1 1 1] 初始化当前路径上Passer X长度缩放系数
      (LocalVariables|SetRandom%20X%20Scale (Math|Float|Lerp 1.0 (Variables|Passer|GetPasser%20Hard) (Math|Random|RandomFloat))))
    (:then_1
      ;[1 1 1] 初始化当前路径上Passer X长度缩放系数
      (LocalVariables|SetPasser%20X%20%20Len (* (LocalVariables|GetRandom%20X%20Scale) (.x (Variables|Passer|GetPasser%20XYZ)))))
    (:then_2
      ;[1 1 1] 根据基准点 初始化Passer  生成点
      (bind _output_get (LocalVariables|SetPasser%20Start%20Point (Variables|Passer|GetPasser%20Spawn%20Base%20Point)))
      (LocalVariables|SetPasser%20End%20Point (+ _output_get (Math|Vector|MakeVector (LocalVariables|GetPasser%20X%20%20Len) 0.0 0.0))))
    (:then_3
      ;[1 1 1] 如果在X域上超过了最大范围 则停止生成
      (if (> (.X (Math|Vector|BreakVector (LocalVariables|GetPasser%20End%20Point))) (+ (.x (Variables|Point|GetBase%20Point)) (* (.x (Variables|Path|GetPath%20XYZ)) 2.0)))
        (Variables|Default|SetPasser%20Spawn%20Loop false)
        (return)))
    (:then_4
      ;[1 1 1] 销毁通路上的障碍物
      (bind (_outhits _returnvalue) (Class|KismetSystemLibrary|BoxTraceMulti (LocalVariables|GetPasser%20Start%20Point) (LocalVariables|GetPasser%20End%20Point) (Math|Vector|MakeVector 0.0 (.y _passer_xyz) (.z _passer_xyz)) "0, 0, 0" "TraceTypeQuery1" false 0 "None" true "(R=1.000000,G=0.000000,B=0.000000,A=1.000000)" "(R=0.000000,G=1.000000,B=0.000000,A=1.000000)" 1111.0))
      (if _returnvalue
        (for _array_element _outhits
          (Actor|DestroyActor (.HitActor (Collision|BreakHitResult _array_element))))))
    (:then_6
      ;[1 1 1] 设置下一个车道 X 应该偏移多少
      (LocalVariables|SetNext%20X (Math|Float|Lerp (.X (Math|Vector|BreakVector (LocalVariables|GetPasser%20Start%20Point))) (- (.X (Math|Vector|BreakVector (LocalVariables|GetPasser%20End%20Point))) (.x (Variables|Passer|GetPasser%20XYZ))) (Math|Float|SelectFloat (Math|Random|RandomFloat) 1.0 (< (Math|Random|RandomFloat) (Variables|Passer|GetPasser%20Repeat%20Rate))))))
    (:then_7
      ;[1 1 1] 初始化下次生成的基准点
      (Path|RangdomtoPath)
      (Variables|Passer|SetPasser%20Spawn%20Base%20Point (Math|Vector|MakeVector (LocalVariables|GetNext%20X) (Path|GetCurrenPathY) (.Z (Math|Vector|BreakVector (LocalVariables|GetPasser%20End%20Point)))))
      (return))))

(fn GetStartPoint
  (return (Variables|Point|GetCenter%20%20Start%20Point)))

(fn PathMove
  (params (Span :type Integer))
  (if (< (+ Span (Variables|Path|GetCurrent%20Path%20N)) 0)
    (Variables|Path|SetCurrent%20Path%20N 0)
    (elif (>= (+ Span (Variables|Path|GetCurrent%20Path%20N)) (Variables|Path|GetPath%20N))
      (Variables|Path|SetCurrent%20Path%20N (- (Variables|Path|GetPath%20N) 1))
      (else
        (Variables|Path|SetCurrent%20Path%20N (+ Span (Variables|Path|GetCurrent%20Path%20N))))))
  (return (Variables|Path|GetCurrent%20Path%20N) (Path|GetCurrenPathY)))

(fn ToCenterPath
  (Variables|Path|SetCurrent%20Path%20N (Variables|Path|GetCenter%20Path%20N)))